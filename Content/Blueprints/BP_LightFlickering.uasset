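; BP_LightFlickering is a Blueprint that drives a sine material on a sphere, apparently as a flickering-light study.
; BeginPlay creates a dynamic instance of M_StudySine_Position and applies it to the sphere.
; Tick remaps a sine to the 0–1 range, prints it and writes it to the SineFrequency parameter.
; The sine takes frame delta rather than accumulated time, so the value stays nearly constant at steady frame rates.
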(event EventTick
  (params (DeltaSeconds :type Float%20%28single-precision%29))
  (bind _returnvalue (|(sin(x)) DeltaSeconds))
  (bind _returnvalue_2 (* _returnvalue 0.5))
  (bind _returnvalue_3 (+ _returnvalue_2 0.5))
  (Development|PrintString (Utilities|String|ToString(Float) _returnvalue_3))
  (Rendering|Material|SetScalarParameterValue (stale EventBeginPlay _output_get) "SineFrequency" _returnvalue_3 :!class /Script/Engine.MaterialInstanceDynamic))

(event EventBeginPlay
  (bind _returnvalue (Rendering|Material|CreateDynamicMaterialInstance (Variables|Default|GetSphere) 0 "/Game/Materials/StudyMaterials/TechArtAid/M_StudySine_Position.M_StudySine_Position" "None" :!class /Script/Engine.PrimitiveComponent))
  (bind _output_get (Variables|Default|SetNewVar _returnvalue))
  (Rendering|Material|SetMaterial (Variables|Default|GetSphere) 0 _output_get))

(fn ConstructionScript)