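; Traversable level-design box that supplies motion warp points for traversal moves such as vaulting or climbing.
; The construction script builds four ledge splines along the top edges from BoxSize and maps opposite pairs and direction vectors.
; GetMotionPoints finds the ledge nearest a hit, then returns points on it and its opposite, clamped by MinLedgeWidth, plus TraversableType.
; A separate GetClosestSpline ranks ledges by dot product and prints debug text.
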(fn `GetClosestSpline`
  (params (IN_ImpactPosition :type "Vector Structure"))
  (returns (OUT_ClosestSpline :type "SplineComponent Object Reference"))
  (locals (ClosestDistanceValue :type "SplineComponent Object Reference") (CurrentMinimumDistance :type "Float (double-precision)" :default 2000.0))
  (set `local.CurrentMinimumDistance` 0.0)
  (set `local.ClosestDistanceValue` null)
  (for _array_element (`self.Ledges`)
    (bind _returnvalue (`KismetMathLibrary.Dot_VectorVector` (`SceneComponent.K2_GetComponentLocation` _array_element) (`local.IN_ImpactPosition`)))
    (if (> _returnvalue (`local.CurrentMinimumDistance`))
      (set `local.CurrentMinimumDistance` _returnvalue)
      (set `local.ClosestDistanceValue` _array_element)
      (`KismetSystemLibrary.PrintString` (`KismetStringLibrary.Concat_StrStr` (`KismetSystemLibrary.GetDisplayName` _array_element) " - " (`KismetStringLibrary.Conv_DoubleToString` _returnvalue)) true true (struct :`G` 1.0 :`B` 0.167573 :`A` 1.0) 5.0)))
  (return (`local.ClosestDistanceValue`)))

(fn `GetMotionPoints`
  (params (IN_HitActor :type "HitResult Structure"))
  (returns (OUT_MotionWarpPoints :type "Array of Vector Structure") (OUT_TraversableType :type "/Game/PlaygroundGAS/Blueprints/Interfaces/ETraversableType Enum"))
  (locals (OUT_Ledge :type "SplineComponent Object Reference") (MinLedgeWidth :type "Float (double-precision)" :default 60.0) (ClosestDistance :type "Float (double-precision)"))
  (bind _out_ledge (`local.OUT_Ledge`))
  (bind (_bblockinghit _binitialoverlap _time _distance _location _impactpoint) (`GameplayStatics.BreakHitResult` (`local.IN_HitActor`)))
  (bind (_value _returnvalue) (`BlueprintMapLibrary.Map_Find` (`self.OppositeLedges`) (`local.OUT_Ledge`)))
  (bind _returnvalue_2 (/ (`local.MinLedgeWidth`) 2.0))
  (bind _returnvalue_3 (/ (`local.MinLedgeWidth`) 2.0))
  (bind _returnvalue_location (`KismetMathLibrary.BreakTransform` (`SplineComponent.GetTransformAtDistanceAlongSpline` _value (`KismetMathLibrary.FClamp` (`SplineComponent.GetDistanceAlongSplineAtLocation` _value (`SplineComponent.FindLocationClosestToWorldLocation` _value _impactpoint "Local") "Local") _returnvalue_2 (- (`SplineComponent.GetSplineLength` _value) _returnvalue_2)) "World" false)))
  (bind (_returnvalue_location_2 _returnvalue_rotation) (`KismetMathLibrary.BreakTransform` (`SplineComponent.GetTransformAtDistanceAlongSpline` _out_ledge (`KismetMathLibrary.FClamp` (`SplineComponent.GetDistanceAlongSplineAtLocation` _out_ledge (`SplineComponent.FindLocationClosestToWorldLocation` _out_ledge _impactpoint "Local") "Local") _returnvalue_3 (- (`SplineComponent.GetSplineLength` _out_ledge) _returnvalue_3)) "World" false)))
  (for (_array_element _array_index) (`self.Ledges`)
    (bind _returnvalue_4 (`KismetMathLibrary.Vector_Distance` (+ (`SplineComponent.FindLocationClosestToWorldLocation` _array_element _impactpoint "World") (* (`SplineComponent.FindUpVectorClosestToWorldLocation` _array_element _impactpoint "World") 10.0)) _impactpoint))
    (if (or (< _returnvalue_4 (`local.ClosestDistance`)) (== _array_index 0))
      (set `local.ClosestDistance` _returnvalue_4)
      (set `local.OUT_Ledge` _array_element)))
  (if _returnvalue
    (return (`|MakeArray` _returnvalue_location_2 _returnvalue_location) (`self.TraversableType`))))

(fn `UserConstructionScript`
  (bind (_boxsize_x _boxsize_y _boxsize_z) (`KismetMathLibrary.BreakVector` (`self.BoxSize`)))
  (bind (_boxsize_x_2 _boxsize_y_2 _boxsize_z_2) (`KismetMathLibrary.BreakVector` (`self.BoxSize`)))
  (bind (_boxsize_x_3 _boxsize_y_3 _boxsize_z_3) (`KismetMathLibrary.BreakVector` (`self.BoxSize`)))
  (bind (_boxsize_x_4 _boxsize_y_4 _boxsize_z_4) (`KismetMathLibrary.BreakVector` (`self.BoxSize`)))
  (`parent.UserConstructionScript`)
  (`SplineComponent.SetSplinePoints` (`self.Ledge_1`) (`|MakeArray` (`KismetMathLibrary.MakeVector` 0.0 _boxsize_y_4 _boxsize_z_4) (`KismetMathLibrary.MakeVector` _boxsize_x_4 _boxsize_y_4 _boxsize_z_4) :!type "Vector Structure") "Local" true)
  (`SplineComponent.SetSplinePoints` (`self.Ledge_2`) (`|MakeArray` (`KismetMathLibrary.MakeVector` 0.0 0.0 _boxsize_z_3) (`KismetMathLibrary.MakeVector` _boxsize_x_3 0.0 _boxsize_z_3) :!type "Vector Structure") "Local" true)
  (`SplineComponent.SetSplinePoints` (`self.Ledge_3`) (`|MakeArray` (`KismetMathLibrary.MakeVector` 0.0 0.0 _boxsize_z_2) (`KismetMathLibrary.MakeVector` 0.0 _boxsize_y_2 _boxsize_z_2) :!type "Vector Structure") "Local" true)
  (`SplineComponent.SetSplinePoints` (`self.Ledge_4`) (`|MakeArray` (`KismetMathLibrary.MakeVector` _boxsize_x 0.0 _boxsize_z) (`KismetMathLibrary.MakeVector` _boxsize_x (/ _boxsize_y 2.0) _boxsize_z) (`KismetMathLibrary.MakeVector` _boxsize_x _boxsize_y _boxsize_z) :!type "Vector Structure") "Local" true)
  (set `self.Ledges` (`|MakeArray` (`self.Ledge_1`) (`self.Ledge_2`) (`self.Ledge_3`) (`self.Ledge_4`)))
  (set `self.OppositeLedges` (`|MakeMap` (`self.Ledge_1`) (`self.Ledge_2`) (`self.Ledge_2`) (`self.Ledge_1`) (`self.Ledge_3`) (`self.Ledge_4`) (`self.Ledge_4`) (`self.Ledge_3`)))
  (set `self.LedgeVectors` (`|MakeMap` (`self.Ledge_1`) (1.0 0.0 0.0) (`self.Ledge_2`) (-1.0 0.0 0.0) (`self.Ledge_3`) (0.0 1.0 0.0) (`self.Ledge_4`) (0.0 -1.0 0.0) :!valuetype "Vector Structure")))