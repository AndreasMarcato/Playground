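; BP_PooledActor is an actor meant for object pooling, switched between active and dormant states instead of being destroyed.
; SetInUse toggles collision, visibility and tick together, and the actor starts dormant on BeginPlay.
; Activation restarts a time-to-live timer that calls ReturnToPool, which deactivates the actor when the time runs out.
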(event `self.ReceiveBeginPlay`
  (`self.SetInUse` false))

(event `SetInUse`
  (params (bIsInUse :type Boolean))
  (bind _output_get (set `self.bIsInUse` bIsInUse))
  (`self.SetActorEnableCollision` _output_get)
  (`self.SetActorHiddenInGame` (not _output_get))
  (`self.SetActorTickEnabled` _output_get)
  (`KismetSystemLibrary.K2_ClearAndInvalidateTimerHandle` (`self.TimeToLiveTimer`))
  (if _output_get
    (bind _returnvalue (`KismetSystemLibrary.K2_SetTimerDelegate` (delegate `ReturnToPool`) (`self.TimeToLive`)))
    (set `self.TimeToLiveTimer` _returnvalue)))

(event `ReturnToPool`
  (`self.SetInUse` false))

(fn `UserConstructionScript`)