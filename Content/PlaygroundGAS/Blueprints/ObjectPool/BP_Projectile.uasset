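; BP_Projectile is a pooled projectile that is switched on and off through an overridden SetInUse event.
; When in use it flies along its forward vector at fixed speed with its NS effect active; when released it zeroes velocity and deactivates the effect.
; On overlap with an actor tagged ColliderProjectile, it spawns an impact emitter and sound, then marks itself unused instead of being destroyed.
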(event `self.SetInUse`
  (params (bIsInUse :type Boolean))
  (bind _projectilemovement (`self.ProjectileMovement`))
  (bind _ns (`self.NS`))
  (`parent.SetInUse` bIsInUse)
  (if bIsInUse
    (set `MovementComponent.Velocity` (* (`self.GetActorForwardVector`) 700.0) _projectilemovement)
    (`ActorComponent.Activate` _ns true)
    (else
      (set `MovementComponent.Velocity` (0.0 0.0 0.0) _projectilemovement)
      (`ActorComponent.Deactivate` _ns))))

(event `self.ReceiveBeginPlay`)

(event `self.ReceiveActorBeginOverlap`
  (params (OtherActor :type "Actor Object Reference"))
  (bind _returnvalue (`self.K2_GetActorLocation`))
  (if (`self.ActorHasTag` OtherActor "ColliderProjectile")
    (`GameplayStatics.SpawnEmitterAtLocation` null _returnvalue)
    (`GameplayStatics.PlaySoundAtLocation` null _returnvalue (struct) 1.0 1.0 0.0 null null null null)
    (`self.SetInUse` false)))

(fn `UserConstructionScript`)