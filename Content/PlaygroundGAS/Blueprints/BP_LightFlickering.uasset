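; BP_LightFlickering is a Blueprint that drives a sine-based material on its Sphere, apparently as a flicker effect.
; On BeginPlay it creates a dynamic instance of M_StudySine_Position and assigns it to the sphere.
; Each Tick it sets the SineFrequency parameter to a sine of DeltaSeconds remapped to 0–1.
; The sine takes frame delta rather than accumulated time, so the value varies only with frame time.
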(event EventTick
  (params (DeltaSeconds :type Float%20%28single-precision%29))
  (Rendering|Material|SetScalarParameterValue (stale EventBeginPlay _output_get) "SineFrequency" (+ (* (|(sin(x)) DeltaSeconds) 0.5) 0.5) :!class /Script/Engine.MaterialInstanceDynamic))

(event EventBeginPlay
  (bind _returnvalue (Rendering|Material|CreateDynamicMaterialInstance (Variables|Default|GetSphere) 0 "/Game/Materials/StudyMaterials/TechArtAid/M_StudySine_Position.M_StudySine_Position" "None" :!class /Script/Engine.PrimitiveComponent))
  (bind _output_get (Variables|Default|SetNewVar _returnvalue))
  (Rendering|Material|SetMaterial (Variables|Default|GetSphere) 0 _output_get))

(fn ConstructionScript)