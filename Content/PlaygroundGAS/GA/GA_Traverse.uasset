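; Gameplay Ability for contextual traversal that falls back to a normal jump when nothing traversable is ahead of the avatar.
; Box-traces forward, then asks a BPI_Traversable hit actor for its traversal type and motion warp points.
; Traversal is unfinished: Vault 1m only draws debug spheres at those points, and the other types are empty.
; The ability ends immediately after either path, with no montage or warping applied.
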(event `self.K2_ActivateAbility`
  (bind _returnvalue (`self.GetAvatarActorFromActorInfo`))
  (bind _returnvalue_2 (`Actor.K2_GetActorLocation` _returnvalue))
  (set `self.Hit Actor` null)
  (bind _outhit (`KismetSystemLibrary.BoxTraceSingle` _returnvalue_2 (+ _returnvalue_2 (* (`Actor.GetActorForwardVector` _returnvalue) 200.0)) (10.0 10.0 40.0) (`Actor.K2_GetActorRotation` _returnvalue) "TraceTypeQuery1" false (`|MakeArray` (`self.GetAvatarActorFromActorInfo`)) "ForOneFrame"))
  (set `self.Out Hit` _outhit)
  (bind (_bblockinghit _binitialoverlap _time _distance _location _impactpoint _normal _impactnormal _physmat _hitactor) (`GameplayStatics.BreakHitResult` _outhit))
  (set `self.Hit Actor` _hitactor)
  (if (`KismetSystemLibrary.DoesImplementInterface` _hitactor "/Game/PlaygroundGAS/Blueprints/Interfaces/BPI_Traversable.BPI_Traversable_C")
    (bind (_out_motionwarppoints _out_traversabletype) (message `/Game/PlaygroundGAS/Blueprints/Interfaces/BPI_Traversable.GetMotionPoints` (`self.Hit Actor`) (`self.Out Hit`)))
    (switch `/Game/PlaygroundGAS/Blueprints/Interfaces/ETraversableType` _out_traversabletype
      (:`NewEnumerator0`
        (for (_array_element _array_index) _out_motionwarppoints
          (`KismetSystemLibrary.DrawDebugSphere` _array_element 10.0 12 (select `int` _array_index :`0` (struct :`R` 0.672443 :`G` 0.109462 :`B` 1.0 :`A` 1.0) :`1` (struct :`R` 1.0 :`G` 1.0 :`A` 1.0) :!type "LinearColor Structure") 2.0 2.0)))
      (:`NewEnumerator1`
        _)
      (:`NewEnumerator2`
        _)
      (:`NewEnumerator3`
        _)
      (:`NewEnumerator4`
        _))
    (`self.K2_EndAbility`)
    (else
      (bind _asbp_character_base_gas (cast `/Game/PlaygroundGAS/Blueprints/Character/BP_CharacterBaseGAS` (`self.GetAvatarActorFromActorInfo`)))
      (`Character.Jump` _asbp_character_base_gas)
      (`self.K2_EndAbility`))))